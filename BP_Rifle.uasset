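; BP_Rifle is the player's first-person rifle, firing bullet actors through a Fire event.
; Fire casts player zero to BP_FirstPersonCharacter and plays a shoot montage on its arms.
; An Arrow component marks the muzzle, providing the BP_Bullet spawn transform and the attach point for the muzzle flash system.
; A gunshot sound plays at the rifle's location, and nothing fires if the cast fails.
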(event Custom|Fire
  (bind _asbp_first_person_character (Utilities|Casting|CastToBP_FirstPersonCharacter (Game|GetPlayerCharacter 0)))
  (Animation|Montage|MontagePlay (Components|SkeletalMesh|GetAnimInstance (Variables|/Game/FirstPerson/Blueprints/BP_FirstPersonCharacter.BP_FirstPersonCharacter_C|GetArms _asbp_first_person_character)) "/Game/FirstPersonArms/Animations/FP_Rifle_Shoot_Montage.FP_Rifle_Shoot_Montage" 1.0 "MontageLength" 0.0 true)
  (Game|SpawnActorfromClass "/Game/FirstPerson/Blueprints/BP_Bullet.BP_Bullet_C" (Transformation|GetWorldTransform (Variables|Default|GetArrow)) "Undefined" "MultiplyWithRoot" 0 0)
  (Audio|PlaySoundatLocation "/Game/ScifiWeapons/Audio/Weapons_Rifle2_Punch_04.Weapons_Rifle2_Punch_04" (Transformation|GetActorLocation) "0, 0, 0" 1.0 1.0 0.0 0 0 0 0)
  (Niagara|SpawnSystemAttached "/Game/ScifiWeapons/Effects/P_MuzzleFlash.P_MuzzleFlash" (Variables|Default|GetArrow) "None" "0, 0, 0" "0, 0, 0" "KeepRelativeOffset" false))

(fn ConstructionScript)